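; Lightning controller actor for the stylized procedural sky that plays strikes once or in loops with random retrigger delays.
; Each strike randomizes position within a volume and rotation, then a timeline samples a color curve's alpha to drive the Sky's lightning light and color.
; Thunder sound is delayed and faded by camera distance, with Hit and Activated dispatchers fired for other logic.
; The construction script previews the animation at a set time.
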(event Custom|Activate
  (params (Delay :type Float%20%28double-precision%29) (Loops :type Integer))
  (bind _retriggertime (Variables|Bolt|GetRetriggerTime))
  ;[1 1 1] Activate in loop
  (Utilities|FlowControl|Delay Delay)
  (Variables|Bolt|SetActivationLoops Loops)
  (if (!= (Variables|Bolt|GetActivationLoops) 0) :!label _label
    (CallFunction|PlayEffect)
    (if (> (Math|Float|Min(Float) (.x _retriggertime) (.y _retriggertime)) 0.0)
      (Math|Integer|DecrementInt (Variables|Bolt|GetActivationLoops)
        (:%20%20
          (Utilities|FlowControl|Delay (Math|Float|Lerp (.x _retriggertime) (.y _retriggertime) (Math|Random|RandomFloat)))
          (goto _label)))
      (else
        (Variables|Bolt|SetActivationLoops 0)))))

(event Custom|PlayEffect
  (bind _animation (Variables|Bolt|GetAnimation))
  ;[1 1 1] Plays anmation
  (CallFunction|UpdateTransform)
  (CallFunction|SetAnimation true)
  (Utilities|IsValid _animation
    (:Is%20Valid
      (Components|Timeline|SetPlayRate (Variables|Default|GetTimeline) (/ (Variables|Bolt|GetAnimationRate) (.MaxTime (Math|Curves|GetTimeRange _animation))))
      (Utilities|FlowControl|Sequence
        (:then_0
          (bind _alpha (Timeline|Timeline PlayFromStart)
            (:Update
              (CallFunction|UpdateAnimation (* _alpha (.MaxTime (Math|Curves|GetTimeRange (Variables|Bolt|GetAnimation))))))
            (:Finished
              (CallFunction|SetAnimation false))))
        (:then_1
          ;[1 1 1] Audio
          (Utilities|IsValid (Variables|Sound|GetSound)
            (:Is%20Valid
              (bind _distance (CallFunction|GetActorDistance))
              (Utilities|FlowControl|Delay (/ _distance (* (Variables|Sound|GetSoundSpeed) 1e+02)))
              (Audio|PlaySoundatLocation (Variables|Sound|GetSound) (Transformation|GetActorLocation) "0, 0, 0" (* (Math|Float|Clamp(Float) (- 1.0 (/ (- _distance (Variables|Sound|GetSoundFadeDistance)) (Variables|Sound|GetSoundFadeWidth)))) (Variables|Sound|GetSoundVolume)) (Variables|Sound|GetSoundPitch) 0.0 0 0 0 0))))
        (:then_2
          ;[1 1 1] Hit event
          (Utilities|FlowControl|Delay (* (Variables|Bolt|GetAnimationRate) (Variables|Hit|GetHitEventTime)))
          (Default|CallOnHit self))
        (:then_3
          (Default|CallOnActivated self))))))

(event Custom|Deactivate
  (params (StopAnimation :type Boolean))
  ;[1 1 1] Deactivate
  (Variables|Bolt|SetActivationLoops 0)
  (CallFunction|UpdateAnimation 0.0)
  (if StopAnimation
    ;[1 1 1] Plays anmation
    (bind _alpha (Timeline|Timeline Stop)
      (:Update
        (CallFunction|UpdateAnimation (* _alpha (.MaxTime (Math|Curves|GetTimeRange (Variables|Bolt|GetAnimation))))))
      (:Finished
        (CallFunction|SetAnimation false)))))

(event EventBeginPlay
  ;[1 1 1] Cache and ativate
  (|CallParentFunction)
  (Variables|Randomization|SetCachedTransform (Transformation|GetWorldTransform (Variables|Default|GetRandomVolume)))
  (Variables|Randomization|SetCachedRotation (Transformation|GetActorRotation))
  (CallFunction|UpdateAnimation 0.0)
  (if (!= (Variables|Bolt|GetActivationLoops) 0)
    (CallFunction|Activate (Variables|Bolt|GetActivationDelay) (Variables|Bolt|GetActivationLoops))))

(fn ConstructionScript
  (CallFunction|UpdateAnimation (Variables|Bolt|GetPreviewTime)))

(fn UpdateAnimation
  (params (InTime :type Float%20%28double-precision%29))
  (bind _animation (Variables|Bolt|GetAnimation))
  (bind _returnvalue (Math|Curves|GetLinearColorValue _animation InTime))
  (bind _asbp_fast_stylized_procedural_sky (Utilities|Casting|CastTo (Variables|External|GetSky)))
  (CallFunction|UpdateLightningData _asbp_fast_stylized_procedural_sky (* (Variables|External|GetSkyLight) (.a _returnvalue)) (* (.a _returnvalue) (Variables|External|GetNightLight)) (* (Variables|Bolt|GetLightningColor) (* (.a _returnvalue) (.a (Variables|Bolt|GetLightningColor)))))
  (CallFunction|InitLightningData _asbp_fast_stylized_procedural_sky (Transformation|GetActorLocation) (Variables|External|GetRadius) (Variables|External|GetClouds) (Variables|External|GetScattering) (Variables|External|GetSkydomeLight)))

(fn UpdateTransform
  (bind _rotationrange (Variables|Randomization|GetRotationRange))
  (if (Variables|Randomization|GetUseRandomization)
    (Transformation|SetActorLocation (Math|Transform|TransformLocation (Variables|Randomization|GetCachedTransform) (Math|Vector|MakeVector (- (Math|Random|RandomFloat) 0.5) (- (Math|Random|RandomFloat) 0.5) (- (Math|Random|RandomFloat) 0.5))) false true)
    (Transformation|SetActorRotation (Math|Rotator|CombineRotators (Variables|Randomization|GetCachedRotation) (Math|Rotator|MakeRotator (* (.roll _rotationrange) (- (Math|Random|RandomFloat) 0.5)) (* (.pitch _rotationrange) (- (Math|Random|RandomFloat) 0.5)) (* (.yaw _rotationrange) (- (Math|Random|RandomFloat) 0.5)))))))

(fn SetAnimation
  (params (ActivateAnimation :type Boolean))
  (bind _output_get (Variables|Bolt|SetIsAnimating ActivateAnimation))
  (bind _asbp_fast_stylized_procedural_sky (Utilities|Casting|CastTo (Variables|External|GetSky)))
  (CallFunction|InitLightningData _asbp_fast_stylized_procedural_sky (Transformation|GetActorLocation) 1e+02 0.0 0.0 0.0))

(fn GetActorDistance
  (return (Math|Vector|VectorLength (- (Transformation|GetActorLocation) (Camera|GetCameraLocation (Game|GetPlayerCameraManager 0))))))