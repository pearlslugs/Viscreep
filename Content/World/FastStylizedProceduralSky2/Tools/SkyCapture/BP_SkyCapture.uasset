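; Editor tool actor that bakes a cube scene capture of the sky into a static skydome or full sky-sphere texture.
; Construction script sets up a preview material and an M_UnwrapCubemap instance with scale and gamma options, then captures with a show-only actor list.
; The Generate bool acts as a one-shot button, drawing the unwrap material to a render target and saving it as a texture asset.
; The resulting texture feeds the preview mesh's material.
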(event Custom|BakeToSkydome
  (bind _compression (Variables|Default|GetCompression))
  (bind _mipsettings (Variables|Default|GetMipSettings))
  (bind _unwrapmaterial (Variables|Default|GetUnwrapMaterial))
  (if (Variables|Default|GetBakeSphere)
    (Rendering|DrawMaterialtoRenderTarget "/Game/World/FastStylizedProceduralSky2/Tools/SkyCapture/Materials/RT_BakedSkySphere.RT_BakedSkySphere" _unwrapmaterial)
    (bind _returnvalue (Class|KismetRenderingLibrary|RenderTargetCreateStaticTexture2DEditorOnly "/Game/World/FastStylizedProceduralSky2/Tools/SkyCapture/Materials/RT_BakedSkySphere.RT_BakedSkySphere" (Utilities|String|Append (Utilities|String|ToString(Text) (Variables|Default|GetFileName)) "_SkySphere") _compression _mipsettings))
    (Variables|Default|SetSkyPreview _returnvalue)
    (else
      (Rendering|DrawMaterialtoRenderTarget "/Game/World/FastStylizedProceduralSky2/Tools/SkyCapture/Materials/RT_BakedSkydome.RT_BakedSkydome" _unwrapmaterial)
      (bind _returnvalue_2 (Class|KismetRenderingLibrary|RenderTargetCreateStaticTexture2DEditorOnly "/Game/World/FastStylizedProceduralSky2/Tools/SkyCapture/Materials/RT_BakedSkydome.RT_BakedSkydome" (Utilities|String|Append (Utilities|String|ToString(Text) (Variables|Default|GetFileName)) "_SkyDome") _compression _mipsettings))
      (Variables|Default|SetSkyPreview _returnvalue_2))))

(event EventBeginPlay)

(event EventTick
  (params (DeltaSeconds :type Float%20%28single-precision%29)))

(fn ConstructionScript
  (CallFunction|UpdatePreview)
  (CallFunction|InitGenerator)
  (Rendering|Material|SetTextureParameterValue (Variables|Default|GetMaterialInstance) "WorldLayer" (Variables|Default|GetSkyPreview)))

(fn UpdatePreview
  (bind _returnvalue (Rendering|Material|CreateDynamicMaterialInstance (Variables|Default|GetPreview) 0 "/Game/World/FastStylizedProceduralSky2/Materials/MI_StaticSkyDome.MI_StaticSkyDome" "None" :!class /Script/Engine.PrimitiveComponent))
  (bind _output_get (Variables|Default|SetMaterialInstance _returnvalue))
  (Rendering|Material|SetScalarParameterValue _output_get "SkySphereUV" (select (Variables|Default|GetBakeSphere) 1.0 0.0) :!class /Script/Engine.MaterialInstanceDynamic))

(fn InitGenerator
  (bind _returnvalue (Rendering|Material|CreateDynamicMaterialInstance "/Game/World/FastStylizedProceduralSky2/Tools/SkyCapture/Materials/M_UnwrapCubemap.M_UnwrapCubemap" "None" "None" :!class /Script/Engine.KismetMaterialLibrary))
  (Variables|Default|SetUnwrapMaterial _returnvalue)
  (Rendering|Material|SetScalarParameterValue _returnvalue "SkyScale" (select (Variables|Default|GetBakeSphere) 0.5 0.25) :!class /Script/Engine.MaterialInstanceDynamic)
  (Rendering|Material|SetScalarParameterValue _returnvalue "GammaCorrection" (select (Variables|Default|GetGammaCorrection) 1.0 0.0) :!class /Script/Engine.MaterialInstanceDynamic)
  (Variables|/Script/Engine.SceneCaptureComponent|SetShowOnlyActors (Variables|Default|GetCaptureComponentCube) (Utilities|Array|MakeArray 0))
  (Rendering|SceneCapture|CaptureScene (Variables|Default|GetCaptureComponentCube) :!class /Script/Engine.SceneCaptureComponentCube)
  (if (Variables|Default|GetGenerate)
    (CallFunction|BaketoSkydome)
    (Variables|Default|SetGenerate false)))