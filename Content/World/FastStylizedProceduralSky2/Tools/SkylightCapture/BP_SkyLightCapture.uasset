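; Editor tool actor that poses a referenced sky at evenly spaced times of day for skylight cubemap capture with a cube capture component.
; The construction script maps the clamped cubemap index and count onto a 0–12 time range and applies it to the sky while capture mode is on.
; Toggling the mode saves the original time of day, then restores it and recaptures the sky and skylight on exit.
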(event EventBeginPlay)

(event EventTick
  (params (DeltaSeconds :type Float%20%28single-precision%29)))

(fn ConstructionScript
  (bind _sky (Variables|Capture|GetSky))
  (bind _capturecubemapcount (Variables|Capture|GetCaptureCubemapCount))
  (Variables|Capture|SetGenerate false)
  (Variables|/Script/Engine.SceneCaptureComponent|SetShowOnlyActors (Variables|Default|GetCaptureComponentCube) (Utilities|Array|MakeArray 0))
  (Variables|Capture|SetCaptureCubemapIndex (Math|Integer|Min(Integer) (Variables|Capture|GetCaptureCubemapIndex) (Variables|Capture|GetCaptureCubemapCount)))
  (Utilities|IsValid (.Sky (Variables|Capture|GetSky))
    (:Is%20Valid
      (if (Math|Boolean|NotEqual(Boolean) (Variables|Capture|GetCaptureMode) (Variables|Debug|GetCaptureModeActive))
        (Variables|Debug|SetCaptureModeActive (Variables|Capture|GetCaptureMode))
        (if (Variables|Capture|GetCaptureMode)
          ;[1 1 1] Save for capture
          (Variables|Debug|SetCaptureSavedTimeOfDay (Variables|Default|GetTimeOfDay (.Sky (Variables|Capture|GetSky))))
          (switch int _capturecubemapcount :!label _label
            (:Default
              (CallFunction|SetTimeOfDay (.Sky (Variables|Capture|GetSky)) (* (- (Variables|Capture|GetCaptureCubemapIndex) 1) (/ 12.0 (Math|Conversions|ToFloat(Integer) (- _capturecubemapcount 1)))))
              (Variables|Capture|SetCaptureTimeDebug (* (- (Variables|Capture|GetCaptureCubemapIndex) 1) (/ 12.0 (Math|Conversions|ToFloat(Integer) (- _capturecubemapcount 1)))))))
          (else
            ;[1 1 1] Load after capture
            (CallFunction|SetTimeOfDay _sky (Variables|Debug|GetCaptureSavedTimeOfDay))
            (CallFunction|PostConstructionScript _sky)
            (CallFunction|RecaptureSky _sky)
            (CallFunction|UpdateSkyLight _sky)))
        (elif (Variables|Capture|GetCaptureMode)
          (goto _label))))))