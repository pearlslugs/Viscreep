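; NPC character Blueprint for melee combat, supplying one-handed sword attack montages and directional hit reactions to a montage manager component.
; BeginPlay also removes the camera, links combat to stats and resets every body part's health.
; Non-special hit stuns play a random montage chosen by attack position and swing direction, spawn brief blood and count hits.
; Attack requests play only primary montages; head-hiding ragdoll logic is disconnected.
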(event EventBeginPlay
  (CallFunction|InitializeMontageComponent)
  (Components|DestroyComponent (Variables|Default|GetCamera))
  (Class|BaseCombatComponent|SetStatsComponent (Variables|Default|GetCombatComponent) (Variables|Default|GetCharacterStatsComponent))
  (CallFunction|InitializeBodyParts))

(event Collision|EventActorBeginOverlap
  (params (OtherActor :type Actor%20Object%20Reference)))

(event EventTick
  (params (DeltaSeconds :type Float%20%28single-precision%29)))

(event OnHitReactionDecided(CombatComponent)
  (params (InitialReaction :type EHitReactionCatagory%20Enum :default "EHRT_None"))
  (bind (_isspecialattack _swingdirection) (Utilities|GetAttackInfo))
  (switch Utilities|FlowControl|Switch|SwitchonEHitReactionCatagory InitialReaction
    (:EHRT_HitStun
      (if (not _isspecialattack)
        (bind _returnvalue (Class|MontageManagerComponent|GetHitreactionMontgeArray (Variables|Default|GetCharacterMontageManagerComponent) (Utilities|GetIncomingAttacPosition) _swingdirection))
        (Utilities|IsValid (.MontageToPlay (Utilities|Struct|BreakAnimMontageStruct (.OutItem (Utilities|Array|Random _returnvalue))))
          (:Is%20Valid
            (Class|BaseRPGCharacter|PlayRPGMontage (.OutItem (Utilities|Array|Random _returnvalue)))
            (bind _returnvalue_2 (Niagara|SpawnSystematLocation "/Game/VFX/Blood/P_Blood03.P_Blood03" (Utilities|GetIncomingHitLocation)))
            (Utilities|FlowControl|Sequence
              (:then_0
                (Utilities|FlowControl|Delay 0.4)
                (Components|DestroyComponent _returnvalue_2))
              (:then_1
                (Math|Integer|IncrementInt (Variables|Default|GetAmountOfHits)))))
          (:Is%20Not%20Valid
            (Development|PrintString "not valid montage")))))))

(event Custom|InitializeMontageComponent
  (Class|MontageManagerComponent|InitializeAllWeaponMontages (Variables|Default|GetCharacterMontageManagerComponent) (AnimationInit|MakeAllWeaponMontages))
  ;[1 1 1] Do when animation lined graph changes
  (Class|MontageManagerComponent|UpdateCurrentWeaponMontages (Variables|Default|GetCharacterMontageManagerComponent) "EAWST_OneHandedSword")
  (Class|MontageManagerComponent|UpdateHitReactionMontages (Variables|Default|GetCharacterMontageManagerComponent) (Utilities|CreateHitReactions)))

(fn ConstructionScript)

(fn MakePrimaryMontages
  (bind _animmontagestruct (Utilities|Struct|MakeAnimMontageStruct "/Game/Characters/SharedAnimations/OneHandedAnims/Attacks/HighAttacks/Montages/HighAttack_3.HighAttack_3" 1.0 0.0 0.0))
  (bind _animmontagestruct_2 (Utilities|Struct|MakeAnimMontageStruct "/Game/Characters/SharedAnimations/OneHandedAnims/Attacks/HighAttacks/Montages/HighAttack.HighAttack" 1.0 0.0 0.0))
  (bind _animmontagestruct_3 (Utilities|Struct|MakeAnimMontageStruct "/Game/Characters/SharedAnimations/OneHandedAnims/Attacks/HighAttacks/Montages/HighAttack_2.HighAttack_2" 1.0 0.0 0.0))
  (bind _array (Utilities|Array|MakeArray _animmontagestruct_2 _animmontagestruct_3 _animmontagestruct))
  (return (Utilities|Struct|MakeDirectionalMontageStructArrays (Utilities|Array|MakeArray (Utilities|Struct|MakeAnimMontageStruct "/Game/Characters/SharedAnimations/OneHandedAnims/Attacks/LowAttacks/Montages/LowAttackMontage.LowAttackMontage" 1.0 0.0 0.0) (Utilities|Struct|MakeAnimMontageStruct "/Game/Characters/SharedAnimations/OneHandedAnims/Attacks/LowAttacks/Montages/LowAttackMontage_2.LowAttackMontage_2" 1.0 0.0 0.0)) (Utilities|Array|MakeArray (Utilities|Struct|MakeAnimMontageStruct "/Game/Characters/SharedAnimations/OneHandedAnims/Attacks/MidAttacks/Montages/MidAttackMontage1.MidAttackMontage1" 1.0 0.0 0.0) (Utilities|Struct|MakeAnimMontageStruct "/Game/Characters/SharedAnimations/OneHandedAnims/Attacks/MidAttacks/Montages/MidAttackMontage2.MidAttackMontage2" 1.0 0.0 0.0) (Utilities|Struct|MakeAnimMontageStruct "/Game/Characters/SharedAnimations/OneHandedAnims/Attacks/MidAttacks/Montages/MidAttackMontage3.MidAttackMontage3" 1.0 0.0 0.0) (Utilities|Struct|MakeAnimMontageStruct "/Game/Characters/SharedAnimations/OneHandedAnims/Attacks/MidAttacks/Montages/MidAttackMontage4.MidAttackMontage4" 1.0 0.0 0.0)) _array _array _array _array)))

(fn MakeOneHandedWeaponMontages
  (return (Utilities|Struct|MakeWeaponDependantMontages "ECA_None" (Utilities|Map|MakeMap "EAAT_Primary" (AnimationInit|MakePrimaryMontages) "EAAT_Secondary" "" "EAAT_Kick" "" "EAAT_WeaponBash" "") (Utilities|Map|MakeMap "EDD_None" "") (Utilities|Map|MakeMap "EHRT_None" ""))))

(fn MakeAllWeaponMontages
  (return (Utilities|Map|MakeMap "EAWST_OneHandedSword" (AnimationInit|MakeOneHandedWeaponMontages))))

(fn MakeHorizontalHitReactions
  (bind _animmontagestruct (Utilities|Struct|MakeAnimMontageStruct "/Game/Characters/SharedAnimations/HitReactions/LowHitReactions/Montages/LowHitReactionFromLeft.LowHitReactionFromLeft" 1.0 0.0 0.0))
  (bind _animmontagestruct_2 (Utilities|Struct|MakeAnimMontageStruct "/Game/Characters/SharedAnimations/HitReactions/MidHitReactions/Montages/MidHitReactionFromLeft.MidHitReactionFromLeft" 1.0 0.0 0.0))
  (bind _animmontagestruct_3 (Utilities|Struct|MakeAnimMontageStruct "/Game/Characters/SharedAnimations/HitReactions/HighHitReactions/Montages/HeadHitFromLeft.HeadHitFromLeft" 1.0 0.0 0.0))
  (bind _array (Utilities|Array|MakeArray _animmontagestruct))
  (bind _array_2 (Utilities|Array|MakeArray _animmontagestruct_2))
  (bind _array_3 (Utilities|Array|MakeArray _animmontagestruct_3))
  (return (Utilities|Struct|MakeDirectionalMontageStructArrays _array _array_2 _array_3 _array _array_2 _array_3)))

(fn MakeHorizontalRightHitReactions
  (bind _animmontagestruct (Utilities|Struct|MakeAnimMontageStruct "/Game/Characters/SharedAnimations/HitReactions/LowHitReactions/Montages/LowHitReactionFromRight.LowHitReactionFromRight" 1.0 0.0 0.0))
  (bind _animmontagestruct_2 (Utilities|Struct|MakeAnimMontageStruct "/Game/Characters/SharedAnimations/HitReactions/MidHitReactions/Montages/MidHitReactionFromRight.MidHitReactionFromRight" 1.0 0.0 0.0))
  (bind _animmontagestruct_3 (Utilities|Struct|MakeAnimMontageStruct "/Game/Characters/SharedAnimations/HitReactions/HighHitReactions/Montages/HeadHitFromRight.HeadHitFromRight" 1.0 0.0 0.0))
  (bind _array (Utilities|Array|MakeArray _animmontagestruct_3))
  (bind _array_2 (Utilities|Array|MakeArray _animmontagestruct))
  (bind _array_3 (Utilities|Array|MakeArray _animmontagestruct_2))
  (return (Utilities|Struct|MakeDirectionalMontageStructArrays _array_2 _array_3 _array _array_2 _array_3 _array)))

(fn MakeStraightonHitReactions
  (bind _animmontagestruct (Utilities|Struct|MakeAnimMontageStruct "/Game/Characters/SharedAnimations/HitReactions/LowHitReactions/Montages/LowHitReactionFromLeft.LowHitReactionFromLeft" 1.0 0.0 0.0))
  (bind _animmontagestruct_2 (Utilities|Struct|MakeAnimMontageStruct "/Game/Characters/SharedAnimations/HitReactions/LowHitReactions/Montages/LowHitReactionFromRight.LowHitReactionFromRight" 1.0 0.0 0.0))
  (bind _animmontagestruct_3 (Utilities|Struct|MakeAnimMontageStruct "/Game/Characters/SharedAnimations/HitReactions/MidHitReactions/Montages/TorsoHitFront.TorsoHitFront" 1.0 0.0 0.0))
  (bind _animmontagestruct_4 (Utilities|Struct|MakeAnimMontageStruct "/Game/Characters/SharedAnimations/HitReactions/HighHitReactions/Montages/HeadHitStraight.HeadHitStraight" 1.0 0.0 0.0))
  (bind _animmontagestruct_5 (Utilities|Struct|MakeAnimMontageStruct "/Game/Characters/SharedAnimations/HitReactions/HighHitReactions/Montages/HeadHitStraight2.HeadHitStraight2" 1.0 0.0 0.0))
  (bind _array (Utilities|Array|MakeArray _animmontagestruct_4 _animmontagestruct_5))
  (bind _array_2 (Utilities|Array|MakeArray _animmontagestruct_2 _animmontagestruct))
  (bind _array_3 (Utilities|Array|MakeArray _animmontagestruct_3))
  (return (Utilities|Struct|MakeDirectionalMontageStructArrays _array_2 _array_3 _array _array_2 _array_3 _array)))

(fn InitializeBodyParts
  (bind _characterstatscomponent (Variables|Default|GetCharacterStatsComponent))
  (bind _bodypartsmap (Variables|/Script/Viscreep.BaseStatsComponent|GetBodyPartsMap _characterstatscomponent))
  (bind _keys (Utilities|Map|Keys _bodypartsmap))
  (for _array_element _keys
    (Utilities|Map|Add _bodypartsmap _array_element (Utilities|Struct|MakeBodyPartStruct 1e+02 1e+02 _array_element))))

(fn RequestMontageandAttack
  (params (InAttackType :type EAllAttackTypes%20Enum :default "EAAT_None") (CurrentAttackPosition :type EAttackPosition%20Enum :default "EAP_None"))
  (bind _returnvalue (Class|BaseRPGCharacter|GetAttackAnimationandSetCombatState InAttackType CurrentAttackPosition))
  (Utilities|GetIsMontageValid _returnvalue
    (:Is%20Valid
      (Class|CombatComponent|SetSelectedMontage (Variables|Default|GetCombatComponent) _returnvalue)
      (switch Utilities|FlowControl|Switch|SwitchonEAllAttackTypes InAttackType
        (:EAAT_Primary
          (Animation|PlayAnimMontage (.MontageToPlay (Utilities|Struct|BreakAnimMontageStruct (Variables|/Script/Viscreep.CombatComponent|GetSelectedMontage (Variables|Default|GetCombatComponent)))) 1.0 "None"))))))

(fn GetWeaponActorandAcceptAttackParams
  (params (InProgressAttack :type Outgoing%20Attack%20Struct%20Structure))
  (return 0))