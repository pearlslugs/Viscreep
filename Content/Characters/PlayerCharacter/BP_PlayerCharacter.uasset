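; ALS-based player character for lock-on, directional melee combat, wiring together combat, state, input buffer, montage, equipment and stats components.
; Lock-on toggles the sword overlay, linked anim layer and controller-facing movement, and repurposes look input as high/mid/low defense position.
; Buffered inputs and combat component requests trigger positional attack montages, dodges or rolls, and jumps.
; BeginPlay builds montage maps and spawns equipped items, attaching weapons to sockets and initialising their damage and collision.
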(event EventUpdateGeneralState
  (params (InState :type ECharacterGeneralState%20Enum :default "ECGS_None"))
  (Class|CharacterStateComponent|ChangeGeneralCharacterState (Variables|Default|GetCharacterStateComponent) InState))

(event Collision|EventActorBeginOverlap
  (params (OtherActor :type Actor%20Object%20Reference)))

(event EventRotatetoTarget
  (params (ShouldRotate :type Boolean))
  (Variables|Default|SetShouldRotateToTarget ShouldRotate)
  (if (and (Variables|Default|GetShouldRotateToTarget) (Utilities|IsValid (Utilities|GetTargetedActor))) :!label _label
    (Transformation|SetActorRotation (Math|Interpolation|RInterpTo (Transformation|GetActorRotation) (Utilities|GetTargetedActorLookatRotation) 0.1 15.0))
    (Utilities|FlowControl|Delay 0.1)
    (goto _label)))

(event EventOnOverlayModeChanged
  (params (PreviousModeTag :type Gameplay%20Tag%20Structure%20%28by%20ref%29))
  (CallFunction|RefreshOverlayLinkedAnimationLayer)
  (CallFunction|RefreshOverlayObject))

(event EventOnMantlingEnded
  (CallFunction|RefreshOverlayObject))

(event EventOnRagdollingEnded
  (CallFunction|RefreshOverlayObject))

(event EventOnMantlingStarted
  (params (Parameters :type Als%20Mantling%20Parameters%20Structure%20%28by%20ref%29))
  (if (Utilities|Enum|NotEqual(Enum) (.mantlingtype Parameters) "Low")
    (CallFunction|ClearOverlayObject)))

(event EventBeginPlay
  (CallFunction|RefreshOverlayObject)
  (CallFunction|RefreshOverlayLinkedAnimationLayer)
  (bind _asbp_viscreep_player_controller (Utilities|Casting|CastToBP_ViscreepPlayerController (Pawn|GetController)))
  (Variables|Default|SetViscreepPlayerController _asbp_viscreep_player_controller)
  (Class|CombatComponent|Initialize (Variables|Default|GetPlayerCombatComponent) self (Variables|Default|GetViscreepPlayerController))
  (CallFunction|InitializeMontageComponent)
  (CallFunction|InitializeEquipmentComponent))

(event EventOnRagdollingStarted
  (CallFunction|ClearOverlayObject))

(event EventTick
  (params (DeltaSeconds :type Float%20%28single-precision%29)))

(event EventUpdateCombatState
  (params (InCombatState :type ECombatState%20Enum :default "ECS_None"))
  (Class|CharacterStateComponent|UpdateCombatState (Variables|Default|GetCharacterStateComponent) InCombatState))

(event Input|KeyboardEvents|M
  (params (Key :type Key%20Structure))
  (:Pressed
    (Development|PrintString (Utilities|String|ToString(Float) (.Value (Utilities|Map|Find (.damagetypemap (Variables|/Script/Viscreep.BaseStatsComponent|GetStatsWeaponData (Variables|Default|GetCharacterStatsComponent))) "EPDT_Slash"))))))

(event OnGeneralStateChanged(CharacterStateComponent)
  (params (NewState :type ECharacterGeneralState%20Enum :default "ECGS_None"))
  (switch Utilities|FlowControl|Switch|SwitchonECharacterGeneralState NewState))

(event Input|EnhancedActionEvents|EnhancedInputActionIA_LockOn
  (params (ActionValue :type Boolean) (ElapsedSeconds :type Float%20%28double-precision%29) (TriggeredSeconds :type Float%20%28double-precision%29) (InputAction :type Input%20Action%20Object%20Reference :default "/ALS/ALS/Data/Input/IA_LockOn.IA_LockOn")))

(event Input|EnhancedActionEvents|EnhancedInputActionIA_LookMouse
  (params (ActionValue :type Vector%202D%20Structure) (ElapsedSeconds :type Float%20%28double-precision%29) (TriggeredSeconds :type Float%20%28double-precision%29) (InputAction :type Input%20Action%20Object%20Reference :default "/ALS/ALS/Data/Input/IA_LookMouse.IA_LookMouse"))
  (:Triggered
    (Input|RecieveLookInput ActionValue false :!label _label))
  (:Started
    (goto _label))
  (:Ongoing
    (goto _label))
  (:Canceled
    (goto _label))
  (:Completed
    (goto _label)))

(event Input|EnhancedActionEvents|EnhancedInputActionIA_Look
  (params (ActionValue :type Vector%202D%20Structure) (ElapsedSeconds :type Float%20%28double-precision%29) (TriggeredSeconds :type Float%20%28double-precision%29) (InputAction :type Input%20Action%20Object%20Reference :default "/ALS/ALS/Data/Input/IA_Look.IA_Look"))
  (:Triggered
    (Input|RecieveLookInput ActionValue true :!label _label))
  (:Started
    (goto _label))
  (:Ongoing
    (goto _label))
  (:Canceled
    (goto _label))
  (:Completed
    (goto _label)))

(event OnMontageRequeted(PlayerCombatComponent)
  (params (TargetedPosition :type EAttackPosition%20Enum :default "EAP_None") (OutAttackType :type EAllAttackTypes%20Enum :default "EAAT_None"))
  (Combat|RequestMontageandAttack OutAttackType (Variables|/Script/Viscreep.BaseCombatComponent|GetCurrentAttackPosition (Variables|Default|GetPlayerCombatComponent))))

(event OnLockedon(PlayerCombatComponent)
  (params (CurrentlyLockedOn :type Boolean))
  (if CurrentlyLockedOn
    (Class|AlsCharacter|SetOverlayMode "(TagName=\"Als.OverlayMode.OneHandedSword\")")
    (Combat|EnterCombat)
    (else
      (Class|AlsCharacter|SetOverlayMode "(TagName=\"Als.OverlayMode.Default\")")
      (Combat|ExitCombat))))

(event OnBufferConsumed(PlayerInputBufferComponent)
  (params (KeyToConsume :type EBufferKey%20Enum :default "EBK_None"))
  (switch Utilities|FlowControl|Switch|SwitchonEBufferKey KeyToConsume
    (:EBK_PrimaryAttack
      (Combat|RequestMontageandAttack "EAAT_Primary" (Variables|/Script/Viscreep.CombatComponent|GetCurrentAttackPosition (Variables|Default|GetPlayerCombatComponent))))
    (:EBK_Dodge
      (if (Utilities|GetIsCharacterinCombat)
        (Class|BaseRPGCharacter|PlayRPGMontage (Utilities|Struct|MakeAnimMontageStruct (Utilities|GetDodgeMontage) 1.0 0.0 0.0))
        (else
          (Class|AlsCharacterExample|InputRoll))))
    (:EBK_Jump
      ;[1 1 1] if jumping from attack montage consume input, delay the action
      (Class|AlsCharacterExample|InputJump (Class|EnhancedInputLibrary|MakeInputActionValueOfType 1.0 1.0 1.0 "Boolean")))))

(event Custom|InitializeMontageComponent
  (Class|MontageManagerComponent|InitializeAllWeaponMontages (Variables|Default|GetCharacterMontageManagerComponent) (AnimationInit|MakeAllWeaponMontages))
  ;[1 1 1] Do when animation lined graph changes
  (Class|MontageManagerComponent|UpdateCurrentWeaponMontages (Variables|Default|GetCharacterMontageManagerComponent) "EAWST_OneHandedSword")
  (Class|MontageManagerComponent|UpdateHitReactionMontages (Variables|Default|GetCharacterMontageManagerComponent) (Utilities|MakeHitReactionsMap)))

(event EventFakeRootMotion
  (params (Enable :type Boolean) (MovementCurve :type Curve%20Float%20Object%20Reference) (MoveForward :type Boolean) (MoveRight :type Boolean))
  (if Enable
    (Utilities|FlowControl|Sequence
      (:then_0
        (goto _label Open))
      (:then_1
        (Utilities|FlowControl|Gate true :!label _label
          (:Exit
            (Class|AlsCharacterExample|InputMove (Utilities|GetFakeRMMovementValue (Math|Curves|GetFloatValue MovementCurve (Variables|Default|GetFakeRMCurveTime)) MoveForward MoveRight))
            (Utilities|FlowControl|Delay 0.01)
            (Variables|Default|SetFakeRMCurveTime (Math|Float|Clamp(Float) (+ (Variables|Default|GetFakeRMCurveTime) 0.03)))
            (goto _label)))))
    (else
      (Variables|Default|SetFakeRMCurveTime 0.0)
      (goto _label Close))))

(event Custom|InitializeEquipmentComponent
  (Equipment|InitializeEquipment))

(event Custom|InitializeWeapon)

(event Custom|InitializeStats
  (bind _enumvalue (|ForEachECharacterStats)
    (:LoopBody
      (Utilities|Map|Add (Variables|/Script/Viscreep.BaseStatsComponent|GetStatsMap (Variables|Default|GetCharacterStatsComponent)) _enumvalue 1e+01))))

(fn ConstructionScript)

(fn RefreshOverlayLinkedAnimationLayer
  (bind _returnvalue (Utilities|GetLinkedAnimLayer))
  (bind _mesh (Variables|Character|GetMesh))
  (LocalVariables|SetOverlayAnimationInstanceClass (.Value (Utilities|Map|Find (Variables|Default|GetOverlayAnimationInstanceClasses) (Variables|Default|GetOverlayMode))))
  (bind _overlayanimationinstanceclass (LocalVariables|GetOverlayAnimationInstanceClass)
    (:then
      (Components|SkeletalMesh|AnimationBlueprintLinking|LinkAnimClassLayers _mesh _overlayanimationinstanceclass)
      (bind _condition (Class|OverlayInterface|GetIsUpdatable(Message) _returnvalue))
      (if _condition
        (Class|OverlayInterface|Initialize(Message) _returnvalue (Variables|Default|GetPlayerCombatComponent))
        (Development|PrintString "succ")
        (else
          (Development|PrintString "Hello"))))
    (:else
      (Components|SkeletalMesh|AnimationBlueprintLinking|LinkAnimClassLayers _mesh 0))))

(fn AttachOverlayObject
  (params (NewStaticMesh :type Static%20Mesh%20Object%20Reference) (NewSkeletalMesh :type Skeletal%20Mesh%20Object%20Reference) (NewAnimationClass :type Anim%20Instance%20Class%20Reference) (SocketName :type Name) (bUseLeftGunBone :type Boolean))
  (LocalVariables|SetResultSocketName (select (Variables|Default|GetbUseGunBoneForOverlayObjects) (select bUseLeftGunBone (Class|AlsConstants|HandLeftGunVirtualBone) (Class|AlsConstants|HandRightGunVirtualBone)) SocketName))
  (Utilities|FlowControl|Sequence
    (:then_0
      (Components|StaticMesh|SetStaticMesh (Variables|Default|GetOverlayStaticMesh) NewStaticMesh)
      (Transformation|AttachComponentToComponent (Variables|Default|GetOverlayStaticMesh) (Variables|Character|GetMesh) (LocalVariables|GetResultSocketName) "SnapToTarget" "SnapToTarget" "SnapToTarget" true))
    (:then_1
      (Components|SkinnedMesh|SetSkinnedAssetandUpdate (Variables|Default|GetOverlaySkeletalMesh) NewSkeletalMesh true)
      (Class|SkeletalMeshComponent|SetAnimClass (Variables|Default|GetOverlaySkeletalMesh) NewAnimationClass)
      (Transformation|AttachComponentToComponent (Variables|Default|GetOverlaySkeletalMesh) (Variables|Character|GetMesh) (LocalVariables|GetResultSocketName) "SnapToTarget" "SnapToTarget" "SnapToTarget" true))))

(fn ClearOverlayObject
  (Components|StaticMesh|SetStaticMesh (Variables|Default|GetOverlayStaticMesh) 0)
  (Components|SkinnedMesh|SetSkinnedAssetandUpdate (Variables|Default|GetOverlaySkeletalMesh) 0 true)
  (Class|SkeletalMeshComponent|SetAnimClass (Variables|Default|GetOverlaySkeletalMesh)))

(fn RefreshOverlayObject
  (|SwitchGameplayTag (Variables|Default|GetOverlayMode)
    (:Default
      (CallFunction|ClearOverlayObject))
    (:Als.OverlayMode.M4
      (CallFunction|AttachOverlayObject 0 0 0 "M4" false))
    (:Als.OverlayMode.PistolOneHanded
      (CallFunction|AttachOverlayObject 0 0 0 "M9" false :!label _label))
    (:Als.OverlayMode.PistolTwoHanded
      (goto _label))
    (:Als.OverlayMode.Bow
      (CallFunction|AttachOverlayObject 0 0 0 "Bow" true))
    (:Als.OverlayMode.Torch
      (CallFunction|AttachOverlayObject 0 0 0 "Torch" true))
    (:Als.OverlayMode.Binoculars
      (CallFunction|AttachOverlayObject 0 0 0 "Binoculars" false))
    (:Als.OverlayMode.Box
      (CallFunction|AttachOverlayObject 0 0 0 "Box" false))
    (:Als.OverlayMode.Barrel
      (CallFunction|AttachOverlayObject 0 0 0 "Barrel" true))))

(fn SelectMantlingSettings
  (params (MantlingType :type EAlsMantlingType%20Enum :default "High"))
  (switch Utilities|FlowControl|Switch|SwitchonEAlsMantlingType MantlingType
    (:High
      _)
    (:Low
      (|SwitchGameplayTag (Variables|Default|GetOverlayMode)
        (:Default
          (return 0))
        (:Als.OverlayMode.Injured
          _)
        (:Als.OverlayMode.HandsTied
          (return 0))
        (:Als.OverlayMode.M4
          (return 0))
        (:Als.OverlayMode.PistolOneHanded
          (return 0))
        (:Als.OverlayMode.PistolTwoHanded
          (return 0))
        (:Als.OverlayMode.Bow
          _)
        (:Als.OverlayMode.Torch
          _)
        (:Als.OverlayMode.Binoculars
          (return 0))
        (:Als.OverlayMode.Box
          (return 0))
        (:Als.OverlayMode.Barrel
          _))
      (return 0))
    (:InAir
      _))
  (return 0))

(fn RecieveLookInput
  (params (InputValue :type Vector%202D%20Structure) (IsGamePad :type Boolean))
  (if (Utilities|GetIsCharacterinCombat)
    (Utilities|GetShouldChangePositions InputValue IsGamePad
      (:SetHigh
        (LocalVariables|SetLocalDefensePosition "EDP_AttackHigh")
        (Variables|Combat|SetShouldResetDefensePose false)
        (Utilities|Time|ClearTimerbyFunctionName 0 "ResetToMidPosition")
        (Variables|/Script/Viscreep.CombatComponent|SetCurrentDefensePosition (Variables|Default|GetPlayerCombatComponent) (LocalVariables|GetLocalDefensePosition) :!label _label))
      (:SetMid
        (Variables|Combat|SetShouldResetDefensePose true)
        (Utilities|Time|SetTimerbyFunctionName 0 "ResetToMidPosition" 0.2)
        (Development|PrintString "Hello"))
      (:SetLow
        (LocalVariables|SetLocalDefensePosition "EDP_AttackLow")
        (Variables|Combat|SetShouldResetDefensePose false)
        (Utilities|Time|ClearTimerbyFunctionName 0 "ResetToMidPosition")
        (goto _label)))
    (else
      (Class|AlsCharacterExample|InputLookMouse (Utilities|MakeMouseValue InputValue)))))

(fn ResettoMidPosition
  (if (Variables|Combat|GetShouldResetDefensePose)
    (Variables|/Script/Viscreep.CombatComponent|SetCurrentDefensePosition (Variables|Default|GetPlayerCombatComponent) "EDP_AttackMid")))

(fn RequestMontageandAttack
  (params (InAttackType :type EAllAttackTypes%20Enum :default "EAAT_None") (CurrentAttackPosition :type EAttackPosition%20Enum :default "EAP_None"))
  (bind _playercombatcomponent (Variables|Default|GetPlayerCombatComponent))
  (bind _selectedmontage (Variables|/Script/Viscreep.CombatComponent|GetSelectedMontage _playercombatcomponent))
  (bind _montagetoplay (Utilities|Struct|BreakAnimMontageStruct _selectedmontage))
  (if (Utilities|GetCanAttack)
    (bind _returnvalue (Class|BaseRPGCharacter|GetAttackAnimationandSetCombatState InAttackType CurrentAttackPosition))
    (Utilities|GetIsMontageValid _returnvalue
      (:Is%20Valid
        (Class|CombatComponent|SetSelectedMontage (Variables|Default|GetPlayerCombatComponent) _returnvalue)
        (switch Utilities|FlowControl|Switch|SwitchonEAllAttackTypes InAttackType
          (:EAAT_Primary
            (Utilities|IsValid _montagetoplay
              (:Is%20Valid
                (Animation|PlayAnimMontage _montagetoplay 1.0 "None")))))))
    (else
      (Development|PrintString "cant attack"))))

(fn EnterCombat
  (bind _alscharactermovement (Variables|Default|GetAlsCharacterMovement))
  (Variables|Default|SetbUseControllerRotationYaw true)
  (Variables|/Script/Engine.CharacterMovementComponent|SetbUseControllerDesiredRotation _alscharactermovement true)
  (Variables|/Script/Engine.CharacterMovementComponent|SetbOrientRotationToMovement _alscharactermovement false)
  (Variables|/Script/Viscreep.CharacterStateComponent|SetCurrentCharacterGeneralState (Variables|Default|GetCharacterStateComponent) "ECGS_Combat")
  (CallFunction|RefreshOverlayLinkedAnimationLayer)
  (Class|CharacterStateComponent|UpdateCombatState (Variables|Default|GetCharacterStateComponent) "ECS_InCombat")
  (Class|CharacterStateComponent|ChangeGeneralCharacterState (Variables|Default|GetCharacterStateComponent) "ECGS_Combat"))

(fn ExitCombat
  (bind _alscharactermovement (Variables|Default|GetAlsCharacterMovement))
  (Variables|Default|SetbUseControllerRotationYaw false)
  (Variables|/Script/Engine.CharacterMovementComponent|SetbUseControllerDesiredRotation _alscharactermovement false)
  (Variables|/Script/Engine.CharacterMovementComponent|SetbOrientRotationToMovement _alscharactermovement true)
  (Variables|/Script/Viscreep.CharacterStateComponent|SetCurrentCharacterGeneralState (Variables|Default|GetCharacterStateComponent) "ECGS_General")
  (CallFunction|RefreshOverlayLinkedAnimationLayer))

(fn GetDodgeDirection
  (bind _returnvalue (Input|EnhancedActionValues|GetIA_Move))
  (bind (_x _y) (Math|Vector2D|BreakVector2D _returnvalue))
  (if (< _x 0.0)
    (LocalVariables|SetOutDirection "EDD_Left")
    (elif (> _x 0.0)
      (LocalVariables|SetOutDirection "EDD_Right")
      (elif (> _y 0.0)
        (LocalVariables|SetOutDirection "EDD_Forwards")
        (else
          (LocalVariables|SetOutDirection "EDD_Backwards")))))
  (return (LocalVariables|GetOutDirection)))

(fn InitializeEquipment
  (bind _mesh (Variables|Character|GetMesh))
  (bind _mesh_2 (Variables|Character|GetMesh))
  (bind _keys (Utilities|Map|Keys (Utilities|GetEquippedItems)))
  (for _array_element _keys
    (LocalVariables|SetCurrentKey _array_element)
    (bind _asgeneral_item (Utilities|Casting|CastToGeneralItem (.ContainedDataAsset (Utilities|Struct|BreakSlotItemStruct (.Value (Utilities|Map|Find (Utilities|GetEquippedItems) (LocalVariables|GetCurrentKey)))))))
    (bind _output_get (LocalVariables|SetCurrentItem _asgeneral_item))
    (LocalVariables|SetLocalCurrentWeaponData (Variables|/Script/Viscreep.GeneralItem|GetCurrentWeaponData _output_get))
    (LocalVariables|SetSocketName (.OutBoneName (CallFunction|GetSocketTransformandName (LocalVariables|GetCurrentItem))))
    (bind _returnvalue (Game|SpawnActorfromClass (Utilities|GetItemClass (LocalVariables|GetCurrentItem)) (.OutTransform (CallFunction|GetSocketTransformandName (LocalVariables|GetCurrentItem))) "Undefined" 0 0))
    (if (Utilities|Enum|Equal(Enum) (Variables|/Script/Viscreep.GeneralItem|GetItemEquipSlot (LocalVariables|GetCurrentItem)) "EES_WeaponSlot")
      (bind _asweapon_base (Utilities|Casting|CastToWeaponBase _returnvalue)
        (:then
          (Variables|/Script/Viscreep.WeaponBase|SetWeaponData _asweapon_base (LocalVariables|GetLocalCurrentWeaponData))
          (bind _output_get_2 (Variables|Default|SetEquippedRightHandWeapon _asweapon_base))
          (Components|StaticMesh|SetStaticMesh (Variables|/Script/Viscreep.BaseItem|GetItemStaticMesh _output_get_2) "/Game/SwordAnimations/Models/Sword/Sword.Sword")
          (Transformation|AttachComponentToComponent _output_get_2 _mesh_2 (LocalVariables|GetSocketName) "KeepRelative" "KeepRelative" "KeepRelative" true)
          (Transformation|AttachComponentToComponent (Variables|/Script/Viscreep.BaseItem|GetItemStaticMesh _output_get_2) _mesh_2 (LocalVariables|GetSocketName) "KeepRelative" "KeepRelative" "KeepRelative" true)
          (Class|BaseStatsComponent|InitializeWeaponData (Variables|Default|GetCharacterStatsComponent) (Variables|Default|GetEquippedRightHandWeapon) (LocalVariables|GetLocalCurrentWeaponData) 8.0)
          (Class|WeaponCollisionComponent|InitializeStaticMesh (Variables|/Script/Viscreep.WeaponBase|GetWeaponCollision (Variables|Default|GetEquippedRightHandWeapon)) (Variables|/Script/Viscreep.BaseItem|GetItemStaticMesh (Variables|Default|GetEquippedRightHandWeapon)))
          (Class|ActorComponent|SetComponentTickInterval (Variables|/Script/Viscreep.WeaponBase|GetWeaponCollision (Variables|Default|GetEquippedRightHandWeapon)) 0.002))
        (:CastFailed
          (bind _asbase_item (Utilities|Casting|CastToBaseItem _returnvalue :!label _label))
          (Components|StaticMesh|SetStaticMesh (Variables|/Script/Viscreep.BaseItem|GetItemStaticMesh _asbase_item) "/Game/SwordAnimations/Models/Sword/Sword.Sword")
          (Transformation|AttachComponentToComponent _asbase_item _mesh (LocalVariables|GetSocketName) "KeepRelative" "KeepRelative" "KeepRelative" true)
          (Transformation|AttachComponentToComponent (Variables|/Script/Viscreep.BaseItem|GetItemStaticMesh _asbase_item) _mesh (LocalVariables|GetSocketName) "KeepRelative" "KeepRelative" "KeepRelative" true)))
      (else
        (goto _label)))))

(fn GetSocketTransformandName
  (params (InItem :type General%20Item%20Object%20Reference))
  (bind _itemequipslot (Variables|/Script/Viscreep.GeneralItem|GetItemEquipSlot InItem))
  (bind _itemequipsocket (Variables|/Script/Viscreep.GeneralItem|GetItemEquipSocket InItem))
  (bind _returnvalue (Utilities|Select :Index _itemequipsocket :EESO_None "None" :EESO_OneHandedSocket "OneHandedWeaponSocket" :EESO_TwoHandedBaseGripSocket "None" :EESO_TwoHandedPoleGripSocket "None"))
  (bind _returnvalue_2 (Utilities|Select :Index _itemequipslot :EES_Head "None" :EES_Neck "None" :EES_UpperBody "None" :EES_Shoulders "None" :EES_Arms "None" :EES_Hands "None" :EES_Legs "None" :EES_Feet "None" :EES_OffhandTool "None" :EES_WeaponSlot _returnvalue :EES_RingOne "None" :EES_RingTwo "None" :EES_Pendant "None" :EES_BackPack "None" :EES_WaistPack "None"))
  (return (Transformation|GetSocketTransform (Variables|Character|GetMesh) _returnvalue_2 "RTS_World") _returnvalue_2))

(fn MakePrimaryMontages
  (bind _animmontagestruct (Utilities|Struct|MakeAnimMontageStruct "/Game/Characters/SharedAnimations/OneHandedAnims/Attacks/HighAttacks/Montages/HighAttack_3.HighAttack_3" 1.0 0.0 0.0))
  (bind _animmontagestruct_2 (Utilities|Struct|MakeAnimMontageStruct "/Game/Characters/SharedAnimations/OneHandedAnims/Attacks/HighAttacks/Montages/HighAttack.HighAttack" 1.0 0.0 0.0))
  (bind _animmontagestruct_3 (Utilities|Struct|MakeAnimMontageStruct "/Game/Characters/SharedAnimations/OneHandedAnims/Attacks/HighAttacks/Montages/HighAttack_2.HighAttack_2" 1.0 0.0 0.0))
  (bind _array (Utilities|Array|MakeArray _animmontagestruct_2 _animmontagestruct_3 _animmontagestruct))
  (return (Utilities|Struct|MakeDirectionalMontageStructArrays (Utilities|Array|MakeArray (Utilities|Struct|MakeAnimMontageStruct "/Game/Characters/SharedAnimations/OneHandedAnims/Attacks/LowAttacks/Montages/LowAttackMontage.LowAttackMontage" 1.0 0.0 0.0) (Utilities|Struct|MakeAnimMontageStruct "/Game/Characters/SharedAnimations/OneHandedAnims/Attacks/LowAttacks/Montages/LowAttackMontage_2.LowAttackMontage_2" 1.0 0.0 0.0)) (Utilities|Array|MakeArray (Utilities|Struct|MakeAnimMontageStruct "/Game/Characters/SharedAnimations/OneHandedAnims/Attacks/MidAttacks/Montages/MidAttackMontage1.MidAttackMontage1" 1.0 0.0 0.0) (Utilities|Struct|MakeAnimMontageStruct "/Game/Characters/SharedAnimations/OneHandedAnims/Attacks/MidAttacks/Montages/MidAttackMontage2.MidAttackMontage2" 1.0 0.0 0.0) (Utilities|Struct|MakeAnimMontageStruct "/Game/Characters/SharedAnimations/OneHandedAnims/Attacks/MidAttacks/Montages/MidAttackMontage3.MidAttackMontage3" 1.0 0.0 0.0) (Utilities|Struct|MakeAnimMontageStruct "/Game/Characters/SharedAnimations/OneHandedAnims/Attacks/MidAttacks/Montages/MidAttackMontage4.MidAttackMontage4" 1.0 0.0 0.0)) _array _array _array _array)))

(fn MakeOneHandedWeaponMontages
  (return (Utilities|Struct|MakeWeaponDependantMontages "ECA_None" (Utilities|Map|MakeMap "EAAT_Primary" (AnimationInit|MakePrimaryMontages) "EAAT_Secondary" "" "EAAT_Kick" "" "EAAT_WeaponBash" "") (Utilities|Map|MakeMap "EDD_None" "") (Utilities|Map|MakeMap "EHRT_None" ""))))

(fn MakeAllWeaponMontages
  (return (Utilities|Map|MakeMap "EAWST_OneHandedSword" (AnimationInit|MakeOneHandedWeaponMontages))))

(fn MakeHorizontalHitReactions
  (bind _animmontagestruct (Utilities|Struct|MakeAnimMontageStruct "/Game/Characters/SharedAnimations/HitReactions/LowHitReactions/Montages/LowHitReactionFromLeft.LowHitReactionFromLeft" 1.0 0.0 0.0))
  (bind _animmontagestruct_2 (Utilities|Struct|MakeAnimMontageStruct "/Game/Characters/SharedAnimations/HitReactions/MidHitReactions/Montages/MidHitReactionFromLeft.MidHitReactionFromLeft" 1.0 0.0 0.0))
  (bind _animmontagestruct_3 (Utilities|Struct|MakeAnimMontageStruct "/Game/Characters/SharedAnimations/HitReactions/HighHitReactions/Montages/HeadHitFromLeft.HeadHitFromLeft" 1.0 0.0 0.0))
  (bind _array (Utilities|Array|MakeArray _animmontagestruct))
  (bind _array_2 (Utilities|Array|MakeArray _animmontagestruct_2))
  (bind _array_3 (Utilities|Array|MakeArray _animmontagestruct_3))
  (return (Utilities|Struct|MakeDirectionalMontageStructArrays _array _array_2 _array_3 _array _array_2 _array_3)))

(fn MakeHorizontalRightHitReactions
  (bind _animmontagestruct (Utilities|Struct|MakeAnimMontageStruct "/Game/Characters/SharedAnimations/HitReactions/LowHitReactions/Montages/LowHitReactionFromRight.LowHitReactionFromRight" 1.0 0.0 0.0))
  (bind _animmontagestruct_2 (Utilities|Struct|MakeAnimMontageStruct "/Game/Characters/SharedAnimations/HitReactions/MidHitReactions/Montages/MidHitReactionFromRight.MidHitReactionFromRight" 1.0 0.0 0.0))
  (bind _animmontagestruct_3 (Utilities|Struct|MakeAnimMontageStruct "/Game/Characters/SharedAnimations/HitReactions/HighHitReactions/Montages/HeadHitFromRight.HeadHitFromRight" 1.0 0.0 0.0))
  (bind _array (Utilities|Array|MakeArray _animmontagestruct_3))
  (bind _array_2 (Utilities|Array|MakeArray _animmontagestruct))
  (bind _array_3 (Utilities|Array|MakeArray _animmontagestruct_2))
  (return (Utilities|Struct|MakeDirectionalMontageStructArrays _array_2 _array_3 _array _array_2 _array_3 _array)))

(fn MakeStraightonHitReactions
  (bind _animmontagestruct (Utilities|Struct|MakeAnimMontageStruct "/Game/Characters/SharedAnimations/HitReactions/LowHitReactions/Montages/LowHitReactionFromLeft.LowHitReactionFromLeft" 1.0 0.0 0.0))
  (bind _animmontagestruct_2 (Utilities|Struct|MakeAnimMontageStruct "/Game/Characters/SharedAnimations/HitReactions/LowHitReactions/Montages/LowHitReactionFromRight.LowHitReactionFromRight" 1.0 0.0 0.0))
  (bind _animmontagestruct_3 (Utilities|Struct|MakeAnimMontageStruct "/Game/Characters/SharedAnimations/HitReactions/MidHitReactions/Montages/TorsoHitFront.TorsoHitFront" 1.0 0.0 0.0))
  (bind _animmontagestruct_4 (Utilities|Struct|MakeAnimMontageStruct "/Game/Characters/SharedAnimations/HitReactions/HighHitReactions/Montages/HeadHitStraight.HeadHitStraight" 1.0 0.0 0.0))
  (bind _animmontagestruct_5 (Utilities|Struct|MakeAnimMontageStruct "/Game/Characters/SharedAnimations/HitReactions/HighHitReactions/Montages/HeadHitStraight2.HeadHitStraight2" 1.0 0.0 0.0))
  (bind _array (Utilities|Array|MakeArray _animmontagestruct_4 _animmontagestruct_5))
  (bind _array_2 (Utilities|Array|MakeArray _animmontagestruct_2 _animmontagestruct))
  (bind _array_3 (Utilities|Array|MakeArray _animmontagestruct_3))
  (return (Utilities|Struct|MakeDirectionalMontageStructArrays _array_2 _array_3 _array _array_2 _array_3 _array)))

(fn GetWeaponActorandAcceptAttackParams
  (params (InProgressAttack :type Outgoing%20Attack%20Struct%20Structure))
  (Utilities|IsValid (Variables|Default|GetEquippedRightHandWeapon)
    (:Is%20Valid
      (Class|BaseStatsComponent|StoreCurrentAttackInfo (Variables|Default|GetCharacterStatsComponent) InProgressAttack)
      (return (Variables|Default|GetEquippedRightHandWeapon)))
    (:Is%20Not%20Valid
      (Development|PrintString "not valid anymore"))))